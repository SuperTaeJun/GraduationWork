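; Procedural block prop apparently meant to be carved by bullet holes, though the hole logic is not wired.
; The construction script extracts and vertex-colors sculpture, block and hole meshes, but builds only the block as a procedural mesh with collision.
; SetHole is empty; its disconnected nodes randomize hole vertices, apply a mesh boolean to the block and rebuild the section.
; Tick and other events do nothing.
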(event EventBeginPlay)

(event Collision|EventActorBeginOverlap
  (params (OtherActor :type Actor%20Object%20Reference)))

(event EventTick
  (params (DeltaSeconds :type Float%20%28single-precision%29)))

(fn ConstructionScript
  (bind _meshdataa (Variables|Default|GetMeshDataA))
  (Class|BulletHoleWall|GetMeshDatafromStaticMesh "/Game/BreakoutAsset/BulletHole/SM_Scul.SM_Scul" (Variables|Default|GetSculptureData) 0 0 false)
  (Class|BulletHoleWall|SetColorData (Variables|Default|GetSculptureData) "(R=0.662500,G=0.052704,B=0.105497,A=1.000000)")
  (Class|BulletHoleWall|GetMeshDatafromStaticMesh "/Game/BP/GameProp/block3.block3" (Variables|Default|GetMeshDataA) 0 0 false)
  (Class|BulletHoleWall|SetColorData (Variables|Default|GetMeshDataA) "(R=0.662500,G=0.052704,B=0.105497,A=1.000000)")
  (Class|BulletHoleWall|GetMeshDatafromStaticMesh "/Game/BreakoutAsset/BulletHole/SM_BulletHole.SM_BulletHole" (Variables|Default|GetMeshDataB) 0 0 false)
  (Class|BulletHoleWall|SetColorData (Variables|Default|GetMeshDataB) "(R=0.541667,G=0.155340,B=0.198543,A=1.000000)")
  (Class|ProceduralMeshComponent|CreateMeshSectionLinearColor (Variables|Default|GetProceduralMesh) 0 (.verts _meshdataa) (.tris _meshdataa) (.normals _meshdataa) (.uvs _meshdataa) 0 0 0 (.colors _meshdataa) 0 true false)
  (Rendering|Material|SetMaterial (Variables|Default|GetProceduralMesh) 0 "/Game/kjh/M_Block2.M_Block2"))

(fn SetHole
  (params (HitLoc :type Vector)))
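; Escape tool prop that builds a procedural mesh from a source static mesh, apparently prepared for morphing into the JemStoneNew mesh.
; The construction script extracts both meshes, runs UnifyTri on each, then pads the source with collapsed triangles at random vertices toward the gem's vertex count.
; It tints both datasets crimson, stores the source as InterpData and creates the section from it.
; The event graph is empty, so no interpolation runs here.
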(event EventBeginPlay)

(event Collision|EventActorBeginOverlap
  (params (OtherActor :type Actor%20Object%20Reference)))

(event EventTick
  (params (DeltaSeconds :type Float%20%28single-precision%29)))

(fn ConstructionScript
  (bind _data1 (Variables|Default|GetData1))
  (bind _data1_2 (Variables|Default|GetData1))
  (bind _data2 (Variables|Default|GetData2))
  (bind _data1_3 (Variables|Default|GetData1))
  (bind _returnvalue (Utilities|Array|Length (.verts _data1_2)))
  (bind _returnvalue_2 (Utilities|Array|Length (.verts _data2)))
  (Utilities|FlowControl|Sequence
    (:then_0
      (Class|PropBase|GetMeshDatafromStaticMesh (Variables|Default|GetMesh) (Variables|Default|GetData1) 0 0 false)
      (Class|PropBase|UnifyTri (Variables|Default|GetData1))
      (Class|PropBase|GetMeshDatafromStaticMesh "/Game/Maps/MapAsset/jemStoneNew.jemStoneNew" (Variables|Default|GetData2) 0 0 false)
      (Class|PropBase|UnifyTri (Variables|Default|GetData2)))
    (:then_1
      (Utilities|FlowControl|Sequence
        (:then_0
          (if (> _returnvalue_2 _returnvalue)
            (Variables|Default|SetLoopNum (- _returnvalue_2 _returnvalue))
            (for _index (range 0 (- (/ (Variables|Default|GetLoopNum) 3) 1))
              (Variables|Default|SetRandInt (Math|Random|RandomIntegerinRange 0 (- _returnvalue 1)))
              (for _index_2 (range 0 2)
                (Utilities|Array|Add (.tris _data1_2) _returnvalue)
                (Utilities|Array|Add (.verts _data1_2) (Utilities|Array|Get(acopy) (.verts _data1_2) (Variables|Default|GetRandInt)))
                (Utilities|Array|Add (.normals _data1_2) "0,0,1.000000")
                (Utilities|Array|Add :TargetArray (.uvs _data1_2))
                (Utilities|Array|Add :TargetArray (.colors _data1_2))))))))
    (:then_2
      (Class|PropBase|SetColorData _data1_3 "(R=0.662500,G=0.113406,B=0.252090,A=1.000000)")
      (Class|PropBase|SetColorData (Variables|Default|GetData2) "(R=0.662500,G=0.113406,B=0.252090,A=1.000000)")
      (Variables|Default|SetInterpData _data1_3)
      (Class|ProceduralMeshComponent|CreateMeshSectionLinearColor (Variables|Default|GetProceduralMesh) 0 (.verts _data1) (.tris _data1) (.normals _data1) (.uvs _data1) 0 0 0 (.colors _data1) 0 false false)
      (Rendering|Material|SetMaterial (Variables|Default|GetProceduralMesh) 0 (Variables|Default|GetMaterial)))))
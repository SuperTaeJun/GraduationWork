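; BP_EscapeTool is a prop Blueprint that builds a procedural mesh from static mesh data in its Construction Script, with no active gameplay logic.
; It extracts and triangle-unifies data from TESTSHOT2 and TESTRIFLE, then gives both one vertex color.
; Only the TESTSHOT2 data is stored as InterpData and rendered with M_TESTSHOT_Inst.
; Unconnected logic would pad its vertex count toward the rifle's with duplicated vertices, suggesting an unfinished morph.
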(event EventBeginPlay)

(event Collision|EventActorBeginOverlap
  (params (OtherActor :type Actor%20Object%20Reference)))

(event EventTick
  (params (DeltaSeconds :type Float%20%28single-precision%29)))

(fn ConstructionScript
  (bind _data1 (Variables|Default|GetData1))
  (bind _data1_2 (Variables|Default|GetData1))
  (Utilities|FlowControl|Sequence
    (:then_0
      (Class|PropBase|GetMeshDatafromStaticMesh "/Game/BreakoutAsset/Weapon/TEST/TESTSHOT2.TESTSHOT2" (Variables|Default|GetData1) 0 0 false)
      (Class|PropBase|UnifyTri (Variables|Default|GetData1))
      (Class|PropBase|GetMeshDatafromStaticMesh "/Game/BreakoutAsset/Weapon/TEST/TESTRIFLE.TESTRIFLE" (Variables|Default|GetData2) 0 0 false)
      (Class|PropBase|UnifyTri (Variables|Default|GetData2)))
    (:then_2
      (Class|PropBase|SetColorData _data1_2 "(R=0.662500,G=0.113406,B=0.252090,A=1.000000)")
      (Class|PropBase|SetColorData (Variables|Default|GetData2) "(R=0.662500,G=0.113406,B=0.252090,A=1.000000)")
      (Variables|Default|SetInterpData _data1_2)
      (Class|ProceduralMeshComponent|CreateMeshSectionLinearColor (Variables|Default|GetProceduralMesh) 0 (.verts _data1) (.tris _data1) (.normals _data1) (.uvs _data1) 0 0 0 (.colors _data1) 0 false false)
      (Rendering|Material|SetMaterial (Variables|Default|GetProceduralMesh) 0 "/Game/BreakoutAsset/Weapon/TEST/M_TESTSHOT_Inst.M_TESTSHOT_Inst"))))